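; Base harvestable actor that stands in for a PCG instanced mesh, or is hand-placed, and takes damage to yield loot.
; Replicated state drives mesh setup, trace-based removal of the underlying instance and destruction effects, with multicast hit feedback.
; At zero health it spawns drops and a destroy actor, then either self-destructs or times a respawn: hand-placed actors reset, PCG ones return their point and re-add an instance.
; Health and respawn state save to SaveGame.
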(event Custom|CheckInstancedMesh
  ;[1 1 1] Ensures that the instance static mesh is removed on all clients
  (Utilities|IsValid (Variables|/Script/Engine.StaticMeshComponent|GetStaticMesh (Variables|Default|GetStaticMesh))
    (:Is%20Valid
      (Utilities|Time|ClearandInvalidateTimerbyHandle (Variables|Default|GetMeshRemovalTimer))
      (Variables|Default|SetRemoveISM true))))

(event Custom|HitEffect%20%28MC%29
  (params (Position :type Vector) (HitNormal :type Vector))
  ;[1 1 1] Hit Effect
  (CallFunction|PlaySFX(MC) (Variables|Default|GetHitSound) Position)
  (Rendering|Material|SetVectorParameterValue (Variables|Default|GetMat) "Position" (Math|Conversions|ToLinearColor(Vector) Position) :!class /Script/Engine.MaterialInstanceDynamic)
  (bind _newtrack_0 (Timeline|Timeline PlayFromStart)
    (:Update
      (Rendering|Material|SetVectorParameterValue (Variables|Default|GetMat) "Impact" (Math|Conversions|ToLinearColor(Vector) (* HitNormal _newtrack_0)) :!class /Script/Engine.MaterialInstanceDynamic)
      (Rendering|Material|SetScalarParameterValue (Variables|Default|GetMat) "Damage" (- 1.0 (/ (Variables|Default|GetHealth) (Variables|Default|GetMaxHealth))) :!class /Script/Engine.MaterialInstanceDynamic))))

(event Custom|CheckRespawn
  (params (Time :type Float%20%28single-precision%29))
  ;[1 1 1] Respawn Logic
  ;;[1 1 1] Checks if can respawn and starts a respawn timer if it can
  (if (Variables|Default|GetCanRespawn)
    (bind _returnvalue (Utilities|Time|SetTimerbyEvent (delegate Custom|RespawnPCGInstance) Time))
    (Variables|Default|SetRespawnTimer _returnvalue)
    (else
      (Actor|DestroyActor))))

(event Custom|RespawnPCGInstance
  ;[1 1 1] Respawn Logic
  ;;[1 1 1] Checks if can respawn and starts a respawn timer if it can
  (CallFunction|Respawn)
  (if (not (Variables|ManualOverride|GetManuallyPlaced))
    (Utilities|FlowControl|Delay 2.0)
    (Actor|DestroyActor)))

(event Custom|RespawnPCG%20%28MC%29
  (params (NewMesh :type Static%20Mesh%20Object%20Reference))
  (bind _returnvalue (Transformation|GetActorLocation))
  ;[1 1 1] Respawn Logic
  ;;[1 1 1] Multicasts to all clients, checking if an existing mesh already exists and spawning one if it doesn't. This ensures that the actor is respawned as an instanced static mesh for all users.
  (bind _success (CallFunction|GetPCGPartition))
  (if _success
    (Utilities|IsValid (Variables|Default|GetPCGPartition)
      (:Is%20Valid
        (bind _returnvalue_2 (Collision|SphereTraceByChannel _returnvalue _returnvalue 1.5e+02 "TraceTypeQuery5" false 0 "None"))
        (if (not _returnvalue_2)
          (bind _returnvalue_3 (AddComponent|AddInstancedStaticMeshComponent (Variables|Default|GetPCGPartition) false))
          (Components|StaticMesh|SetStaticMesh _returnvalue_3 NewMesh)
          (Components|InstancedStaticMesh|AddInstance _returnvalue_3 (Transformation|GetActorTransform) true))))
    (else
      (Actor|DestroyActor))))

(event Custom|Fade
  ;[1 1 1] Respawn Logic
  (Utilities|IsValid (Variables|Default|GetMat)
    (:Is%20Valid
      (bind _newtrack_0 (Timeline|Timeline_0 PlayFromStart)
        (:Update
          (Rendering|Material|SetScalarParameterValue (Variables|Default|GetMat) "Fade" _newtrack_0 :!class /Script/Engine.MaterialInstanceDynamic))))))

(event Custom|PlaySFX%20%28MC%29
  (params (Sound :type Sound%20Base%20Object%20Reference) (Location :type Vector))
  ;[1 1 1] Respawn Logic
  (Audio|PlaySoundatLocation Sound Location "0, 0, 0" 1.0 1.0 0.0 0 0 0 0))

(event EventSetupHarvestableBPI
  (params (Health :type Float%20%28double-precision%29) (Destroyed :type Boolean) (DestroyClass :type BP%20Chaos%20Destructable%20Master%20Class%20Reference) (RemainingRespawnTime :type Float%20%28double-precision%29) (DropTable :type Data%20Table%20Row%20Handle%20Structure) (PlayerState :type Player%20State%20Object%20Reference) (PCGPoint :type PCG%20Point%20Structure) (Mesh :type Static%20Mesh%20Object%20Reference))
  ;[1 1 1] Sets up the harvestable after spawn
  (CallFunction|SetupHarvestable Health Destroyed DestroyClass RemainingRespawnTime DropTable PlayerState PCGPoint Mesh))

(event EventBeginPlay
  ;[1 1 1] Ensures that the instance static mesh is removed on all clients
  (bind _returnvalue (Utilities|Time|SetTimerbyEvent (delegate Custom|CheckInstancedMesh) 0.01 true))
  (Variables|Default|SetMeshRemovalTimer _returnvalue)
  (if (and (Variables|ManualOverride|GetManuallyPlaced) (not (Variables|Default|GetSetupComplete)))
    (CallFunction|SetupHarvestable :Health -1.0 :Destroy%20Class (Variables|ManualOverride|GetDestroyClassOverride) :DropTable (Variables|ManualOverride|GetDropTableOverride) :Mesh (Variables|ManualOverride|GetMeshOverride)) ; Overrides use if Manually placed is true (Not placed with PCG)
  ))

(event Game|Damage|EventAnyDamage
  (params (Damage :type Float%20%28single-precision%29) (DamageType :type Damage%20Type%20Object%20Reference) (InstigatedBy :type Controller%20Object%20Reference) (DamageCauser :type Actor%20Object%20Reference))
  ;[1 1 1] Applies incoming damage and spawns drop table if destroyed
  (CallFunction|ApplyDamage Damage DamageCauser))

(fn ConstructionScript)

(fn RemoveInstance
  (bind _returnvalue (Transformation|GetActorLocation))
  ;[1 1 1] Does a sphere trace to see if an instance static mesh exists at it's location and removes it if so. Prevents dupes caused by server/client PCG generation
  (bind (_outhit _returnvalue_2) (Collision|BoxTraceByChannel (- _returnvalue "0.000000,0.000000,25.000000") (+ _returnvalue (Math|Vector|MakeVector 1.0 1.0 (* 1e+02 (.z (Transformation|GetActorScale3D))))) (* (.BoxExtent (Collision|GetActorBounds false false)) 0.07) "0, 0, 0" "TraceTypeQuery5" false 0 "None"))
  (if _returnvalue_2
    (bind _asinstanced_static_mesh_component (Utilities|Casting|CastToInstancedStaticMeshComponent (.HitComponent (Collision|BreakHitResult _outhit))))
    (Class|InstancedStaticMeshComponent|RemoveInstance _asinstanced_static_mesh_component (.HitItem (Collision|BreakHitResult _outhit)))
    (Variables|Default|SetInstancedRemoved true)))

(fn SetupHarvestable
  (params (Health :type Float%20%28double-precision%29) (Destroyed :type Boolean) (Destroy%20Class :type BP%20Chaos%20Destructable%20Master%20Class%20Reference) (RemainingRespawnTime :type Float%20%28double-precision%29) (DropTable :type Data%20Table%20Row%20Handle%20Structure) (PlayerState :type Player%20State%20Object%20Reference) (PCGPoint :type PCG%20Point%20Structure) (Mesh :type Static%20Mesh%20Object%20Reference))
  ;[1 1 1] Set required variables on spawn and ensures mesh is correct on all clients. Starts Respawn timer if needs to respawn.
  (Variables|Default|SetSetupComplete true)
  (if (== Health -1.0)
    (Variables|Default|SetHealth (Variables|Default|GetMaxHealth)) ; New Spawn - Use Max Health
    (else
      (Variables|Default|SetHealth Health) ; Loaded - Use Current Health
    ))
  (Variables|Default|SetDefaultMesh Mesh)
  (Variables|Default|SetDestroyed Destroyed)
  (Variables|Default|SetDestroy%20Class Destroy%20Class)
  (Variables|Default|SetDrop%20Table DropTable)
  (Variables|Default|SetPlayer%20State PlayerState)
  (Variables|Default|SetPCGPoint PCGPoint)
  (if (and (> RemainingRespawnTime 0.0) (Variables|Default|GetDestroyed))
    (CallFunction|CheckRespawn RemainingRespawnTime)
    (Variables|Default|SetRemoveISM true)))

(fn ApplyDamage
  (params (Damage :type Float%20%28double-precision%29) (DamageCauser :type Actor%20Object%20Reference))
  ;[1 1 1] Takes the incoming damage and applies it to the object. If destroyed, triggers the spawn table, sets respawn and hides the actor. If not destroyed, updates the UI Hit Display
  (LocalVariables|SetPrevHealth (Variables|Default|GetHealth))
  (Variables|Default|SetHealth (+ (Variables|Default|GetHealth) Damage))
  (if (<= (Variables|Default|GetHealth) 0.0)
    (Variables|Default|SetDestroyed true)
    (Class|BPIPlayerCharacter|SpawnDropTableWorldBPI(Message) DamageCauser (Variables|Default|GetDrop%20Table) (Transformation|GetWorldLocation (Variables|Default|GetLootSpawn)))
    (Game|SpawnActorfromClass (Variables|Default|GetDestroy%20Class) (Transformation|GetWorldTransform (Variables|Default|GetStaticMesh)) "Undefined" "MultiplyWithRoot" 0 (Transformation|GetActorForwardVector DamageCauser) 0)
    (CallFunction|CheckRespawn (Variables|Default|GetRespawnTime)))
  (Class|BPIPlayerCharacter|ShowHitDisplayUIBPI(Message) DamageCauser (Math|Float|Clamp(Float) (/ (LocalVariables|GetPrevHealth) (Variables|Default|GetMaxHealth))) (Math|Float|Clamp(Float) (/ (Variables|Default|GetHealth) (Variables|Default|GetMaxHealth))) (Utilities|Text|ToText(Name) (Variables|Default|GetTable%20ID)) (Variables|Default|GetDestroyed)))

(fn OnRepDestroyed
  (if (Variables|Default|GetDestroyed)
    (Niagara|SpawnSystematLocation (Variables|Default|GetDestroyFX) (+ (Transformation|GetActorLocation) (Variables|Default|GetFXOffset)))
    (CallFunction|Fade)
    (Collision|SetCollisionEnabled (Variables|Default|GetStaticMesh) "NoCollision")
    (CallFunction|PlaySFX(MC) (Variables|Default|GetDestroySound) (Transformation|GetActorLocation))))

(fn GetPCGPartition
  (bind _pcgpoint (Variables|Default|GetPCGPoint))
  (bind _transform (Utilities|Struct|BreakPCGPoint _pcgpoint))
  ;[1 1 1] Does a sphere trace to find the closest instanced static mesh in the area and returns it's PCG Partition parent. If none are found, uses Get Actor Of Class to force one.
  (bind (_outhit _returnvalue) (Collision|SphereTraceByChannel (.location _transform) (.location _transform) 2.5e+04 "TraceTypeQuery5" false 0 "None"))
  (if _returnvalue
    (Variables|Default|SetPCGPartition (.HitActor (Collision|BreakHitResult _outhit)))
    (return true)
    (else
      (bind _returnvalue_2 (Actor|GetActorOfClass "/Script/PCG.PCGPartitionActor"))
      (Utilities|IsValid _returnvalue_2
        (:Is%20Valid
          (Variables|Default|SetPCGPartition _returnvalue_2)
          (return true))
        (:Is%20Not%20Valid
          (return false))))))

(fn Respawn
  ;[1 1 1] After getting the PCG Partition Actor, returns the PCG Point to the Game State to ensure it can be used again.
  (if (Variables|ManualOverride|GetManuallyPlaced)
    (CallFunction|SetupHarvestable :Health -1.0 :Destroy%20Class (Variables|ManualOverride|GetDestroyClassOverride) :DropTable (Variables|ManualOverride|GetDropTableOverride) :Mesh (Variables|ManualOverride|GetMeshOverride)) ; Overrides use if Manually placed is true (Not placed with PCG)
    (Rendering|Material|SetScalarParameterValue (Variables|Default|GetMat) "Fade" 1.0 :!class /Script/Engine.MaterialInstanceDynamic)
    (Collision|SetCollisionEnabled (Variables|Default|GetStaticMesh) "QueryAndPhysics")
    (else
      (Class|BPIGameState|AddPCGPointBPI(Message) (Game|GetGameState) (Variables|Default|GetPCGPoint))
      (CallFunction|RespawnPCG(MC) (Variables|Default|GetDefaultMesh)))))

(fn OnRepDropTable
  (bind _drop_table (Variables|Default|GetDrop%20Table))
  (bind _returnvalue (Utilities|GetDataTableRow (.datatable _drop_table) (.rowname _drop_table))
    (:then
      (Variables|Default|SetTable%20ID (.TableID (Utilities|Struct|BreakSTR_DropTables _returnvalue))))))

(fn OnRepRemoveISM
  (if (not (Variables|Default|GetInstancedRemoved))
    (CallFunction|RemoveInstance)))

(fn OnRepDefaultMesh
  (bind _defaultmesh (Variables|Default|GetDefaultMesh))
  (bind _staticmesh (Variables|Default|GetStaticMesh))
  (Components|StaticMesh|SetStaticMesh (Variables|Default|GetStaticMesh) (select (Variables|Default|GetDestroyed) _defaultmesh _defaultmesh))
  (Utilities|IsValid (Variables|Default|GetDefaultMesh)
    (:Is%20Valid
      (bind _returnvalue (Rendering|Material|CreateDynamicMaterialInstance _staticmesh 0 (Rendering|Material|GetMaterial _staticmesh 0) "None" :!class /Script/Engine.PrimitiveComponent))
      (Variables|Default|SetMat _returnvalue)
      (Rendering|Material|SetMaterial (Variables|Default|GetStaticMesh) 0 (Variables|Default|GetMat)))))

(fn CanbeDamagedBPI
  (params (RepName :type Gameplay%20Tag%20Structure))
  (return (Variables|Default|GetCanBeDamaged)))

(fn CheckFactionBPI
  (params (RepName :type Gameplay%20Tag%20Structure))
  (return "None" false))

(fn CheckInteractableBPI
  (return false 0.0))

(fn CheckIsAliveBPI
  (return false))

(fn CheckTool&RarityBPI
  (return true))

(fn GetDamagingActorNameBPI
  (return "None"))

(fn GetGameDataBPI
  (return 0))

(fn GetGameSettingsSaveDataBPI
  (return false))

(fn GetGUIDBPI
  (return "" "NewEnumerator1"))

(fn GetHarvestableBPI
  ;[1 1 1] Return harvestable reference
  (return self))

(fn GetHitRequirementsBPI
  (return (Variables|Default|GetToolType) (Variables|Default|GetToolRarity)))

(fn GetInteractionTextUIBPI
  (return "" false "0, 0, 0"))

(fn GetLookatServerBPI
  (return false))

(fn GetResistsBPI
  (return 0))

(fn LoadObjectDataBPI
  (params (SaveGame :type BP%20Game%20Save%20Object%20Reference))
  (return true))

(fn SaveObjectDataBPI
  (params (SaveGame :type BP%20Game%20Save%20Object%20Reference))
  ;[1 1 1] Saves all data related to the havestable to the Game Save (Game Mode)
  (Utilities|Array|Add (Variables|/Game/SRPGE/Blueprints/Game/SaveLoad/BP_Game_Save.BP_Game_Save_C|GetHarvestMasters SaveGame) (Utilities|Struct|MakeSTR_SaveGame_HarvestMaster (Utilities|GetClass self) (Transformation|GetActorTransform) (Variables|Default|GetHealth) (Variables|Default|GetDestroyed) (Variables|Default|GetDestroy%20Class) (Utilities|Time|GetTimerRemainingTimebyHandle (Variables|Default|GetRespawnTimer)) (Variables|Default|GetDrop%20Table) (Variables|Default|GetPlayer%20State) (Variables|Default|GetPCGPoint) (Variables|Default|GetDefaultMesh)))
  (return true))

(fn ShouldOutlineBPI
  (return false 1))