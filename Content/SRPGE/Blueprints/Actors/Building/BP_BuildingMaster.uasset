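; Base actor for placeable, replicated building pieces with damage, refund, move highlighting and save support.
; Initializes mesh, destruction class and snap points from DT_Buildings, toggling nearby snaps through sphere traces.
; A box trace links touching pieces as supports and a line trace tags grounded ones.
; On destruction, linked pieces start destroy timers recursively, cancelled back through the graph wherever ground is found; debug modes visualize snaps and support.
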(event `Load&SetMesh`
  (bind ((`BuildMesh_51_EEAD71ED402FF489FF2B99B172EEFD97` _buildmesh)) (break `/Game/SRPGE/Blueprints/Structures/Building/STR_BuildInfo` (`self.BuildInfo`)))
  ;[1 1 1] Loads the building mesh from the soft reference
  (`|LoadAsset` _buildmesh
    (:`Completed`
      (set `self.Build Mesh` (`|ConvertAsset` _buildmesh))
      (`self.CheckSnapPoints` true)
      (`self.SetSupport (Server)`))))

(event `self.ReceiveAnyDamage`
  (params (Damage :type "Float (single-precision)") (DamageType :type "DamageType Object Reference") (InstigatedBy :type "Controller Object Reference") (DamageCauser :type "Actor Object Reference"))
  ;[1 1 1] When damaged
  (if (`self.CanBeDamaged`)
    (bind _destroyed (`self.ApplyDamage` Damage))
    (if _destroyed
      (`self.CheckSnapPoints` false false true)
      (`KismetSystemLibrary.Delay` 0.1)
      (`self.K2_DestroyActor`))))

(event `self.ReceiveBeginPlay`
  ;[1 1 1] Initializes the building
  (set `self.Debug - SetupMode` false) ; Ensures debug is disabled in play
  (`self.InitBuilding(Server)`))

(event `InitBuilding(Server)`
  ;[1 1 1] Initializes the building
  (`self.Init Building`))

(event `SetSupport (Server)`
  (bind _returnvalue (`self.ActorHasTag` "IsOnGround"))
  (bind _origin (`self.GetActorBounds` false))
  (bind (_returnvalue_origin _returnvalue_boxextent) (`KismetMathLibrary.BreakBoxSphereBounds` (`StaticMesh.GetBounds` (`StaticMeshComponent.StaticMesh` (`self.StaticMesh`)))))
  ;[1 1 1] Building Support/Collapse
  ;;[1 1 1] Gets any supporting buildings on creation and adds itself to anything it hits.
  (if (`self.CanTriggerCollapse`)
    (if (`self.Debug - SupportMode`)
      (bind _returnvalue_2 (`AddComponent|NODE_AddStaticMeshComponent-8`))
      (`StaticMeshComponent.SetStaticMesh` _returnvalue_2 (`StaticMeshComponent.StaticMesh` (`self.StaticMesh`)))
      (`PrimitiveComponent.SetCollisionEnabled` _returnvalue_2 "NoCollision")
      (`SceneComponent.SetWorldScale3D` _returnvalue_2 (1.1 1.1 1.1))
      (set `self.DebugSupportMesh` _returnvalue_2))
    (bind _outhits (`KismetSystemLibrary.BoxTraceMulti` _origin _origin (* _returnvalue_boxextent 1.2) (`self.K2_GetActorRotation`) "TraceTypeQuery4"))
    (for _array_element _outhits
      (bind (_bblockinghit _binitialoverlap _time _distance _location _impactpoint _normal _impactnormal _physmat _hitactor) (`GameplayStatics.BreakHitResult` _array_element))
      (`KismetArrayLibrary.Array_AddUnique` (`self.SupportingActors`) _hitactor)
      (bind _asbp_building_master (cast `/Game/SRPGE/Blueprints/Actors/Building/BP_BuildingMaster` _hitactor))
      (`self.UpdateSupportBuildings (Server)` _asbp_building_master self))
    (if (`self.Debug - SupportMode`)
      (`PrimitiveComponent.SetMaterial` (`self.DebugSupportMesh`) 0 (select `bool` _returnvalue :`false` (select `bool` (`KismetArrayLibrary.Array_IsEmpty` (`self.SupportingActors`)) :`false` "/Game/SRPGE/Demo/Assets/Materials/Environment/MI_DebugTransparent_Orange.MI_DebugTransparent_Orange" :`true` "/Game/SRPGE/Demo/Assets/Materials/Environment/MI_DebugTransparent_Red.MI_DebugTransparent_Red" :!type "MaterialInterface Object Reference") :`true` "/Game/SRPGE/Demo/Assets/Materials/Environment/MI_DebugTransparent_green.MI_DebugTransparent_green")))
    (if (not (or _returnvalue (`KismetArrayLibrary.Array_IsNotEmpty` (`self.SupportingActors`))))
      (`self.CollapseSupportCheck (Server)` null 2.0))))

(event `DestroyBuilding (Server)`
  (params (Class :type "Actor Class Reference"))
  ;[1 1 1] When damaged
  (`|SpawnActorFromClass` Class (`self.GetTransform`) "AlwaysSpawn" "MultiplyWithRoot" null null))

(event `SetSnaps (Server)`
  (bind _snappoints (`self.SnapPoints`))
  ;[1 1 1] Passes snap points from the server to the client
  (`self.SetSnaps (Client)` _snappoints)
  (if (not (`self.SnapsChecked`))
    (set `self.CanTriggerCollapse` (`KismetArrayLibrary.Array_IsNotEmpty` _snappoints))
    (set `self.SnapsChecked` true)))

(event `/Game/SRPGE/Blueprints/Interfaces/BPI_Building.SetBuildingManager_BPI`
  (params (BuildingManager :type "/Game/SRPGE/Blueprints/Actors/Building/BP_BuildingManager Object Reference"))
  ;[1 1 1] Sets the building manager
  (`self.SetBuildingManager (Server)` BuildingManager))

(event `SetBuildingManager (Server)`
  (params (BuildingManager :type "/Game/SRPGE/Blueprints/Actors/Building/BP_BuildingManager Object Reference"))
  ;[1 1 1] Sets the building manager
  (set `self.BuildingManager` BuildingManager))

(event `SetSnaps (Client)`
  (params (SnapPoints :type "Array of /Game/SRPGE/Blueprints/Structures/Building/STR_BuildingSnaps Structure"))
  ;[1 1 1] Passes snap points from the server to the client
  (set `self.SnapPoints` SnapPoints))

(event `UpdateSupportBuildings (Server)`
  (params (Actor :type "Actor Object Reference"))
  ;[1 1 1] Building Support/Collapse
  ;;[1 1 1] Gets any supporting buildings on creation and adds itself to anything it hits.
  (`KismetArrayLibrary.Array_AddUnique` (`self.SupportingActors`) Actor))

(event `/Game/SRPGE/Blueprints/Interfaces/BPI_Building.UpdateSnapIsActive_BPI`
  (params (SnapLocation :type "Vector Structure") (IsActive :type Boolean))
  ;[1 1 1] Updates a snap point usage
  (`self.UpdateSnapIsActive (Server)` SnapLocation IsActive))

(event `/Game/SRPGE/Blueprints/Interfaces/BPI_Interaction.TriggerInteraction_BPI`
  (params (PlayerController :type "Controller Object Reference") (PlayerCharacter :type "/Game/SRPGE/Blueprints/Player/BP_PlayerCharacter Object Reference") (BuildRefund :type Boolean))
  ;[1 1 1] Refund and Destroy / Move Building. Triggered when a player chooses to destroy a building.
  (if BuildRefund
    (`self.RefundAndDestroy (Server)` PlayerController)))

(event `SetBuildingRefund (Client)`
  (params (`Can Refund` :type Boolean))
  ;[1 1 1] Refund and Destroy / Move Building. Triggered when a player chooses to destroy a building.
  (set `self.CanRefund` `Can Refund`)
  (if (`self.CanRefund`)
    (if (not (`self.Build Move`))
      (for (_array_element _array_index) (`self.BaseMats`) :!label _label
        (`self.SetMaterial` _array_index (select `bool` (`self.CanRefund`) :`false` _array_element :`true` "/Game/SRPGE/Demo/Assets/Materials/Environment/MI_DebugTransparent_Red.MI_DebugTransparent_Red"))))
    (else
      (set `self.Build Move` false)
      (goto _label))))

(event `/Game/SRPGE/Blueprints/Interfaces/BPI_Building.SetBuildMove_BPI`
  (params (BuildMove :type Boolean))
  ;[1 1 1] Refund and Destroy / Move Building. Triggered when a player chooses to destroy a building.
  (`self.SetBuildMove (Client)` BuildMove))

(event `StartCollapse (Server)`
  (bind _returnvalue (`self.K2_GetActorLocation`))
  ;[1 1 1] Building Support/Collapse
  ;;[1 1 1] Triggers the collaspe on destroy. Does a collapse support check on all actors being supported by this actor.
  (bind _outhits (`KismetSystemLibrary.SphereTraceMulti` _returnvalue _returnvalue 5000.0 "TraceTypeQuery4")) ; If it is the original destroyed object, a sphere trace is used to calulate the collapse timer. This ensures large bases process correctly
  (set `self.CollapseTimer` (* (`KismetArrayLibrary.Array_Length` _outhits) 0.04))
  (for _array_element (`self.SupportingActors`)
    (`/Engine/EditorBlueprintResources/StandardMacros.IsValid` _array_element
      (:`Is Valid`
        (bind _asbp_building_master (cast `/Game/SRPGE/Blueprints/Actors/Building/BP_BuildingMaster` _array_element))
        (`self.CollapseSupportCheck (Server)` _asbp_building_master self (`self.CollapseTimer`))))))

(event `UpdateSnapIsActive (Server)`
  (params (SnapLocation :type "Vector Structure") (Active :type Boolean))
  ;[1 1 1] Updates a snap point usage
  (`self.SetSnapUsed` SnapLocation Active))

(event `/Game/SRPGE/Blueprints/Interfaces/BPI_Building.SetBuildRefund_BPI`
  (params (CanRefund :type Boolean))
  ;[1 1 1] Refund and Destroy / Move Building. Triggered when a player chooses to destroy a building.
  (set `self.CanRefund` CanRefund)
  (`self.SetBuildingRefund (Client)` CanRefund))

(event `self.ReceiveDestroyed`
  ;[1 1 1] Building Support/Collapse
  ;;[1 1 1] Triggers the collaspe on destroy. Does a collapse support check on all actors being supported by this actor.
  (if (`self.CanTriggerCollapse`)
    (`PrimitiveComponent.SetCollisionEnabled` (`self.StaticMesh`) "NoCollision")
    (`self.StartCollapse (Server)`)))

(event `SetBuildMove (Client)`
  (params (BuildMove :type Boolean))
  ;[1 1 1] Refund and Destroy / Move Building. Triggered when a player chooses to destroy a building.
  (set `self.Build Move` BuildMove)
  (set `self.CanRefund` BuildMove)
  (for (_array_element _array_index) (`self.BaseMats`)
    (`self.SetMaterial` _array_index (select `bool` (`self.Build Move`) :`false` _array_element :`true` "/Game/SRPGE/Demo/Assets/Materials/Environment/MI_DebugTransparent_Orange.MI_DebugTransparent_Orange")))
  (`PrimitiveComponent.SetCollisionEnabled` (`self.StaticMesh`) (select `bool` (`self.Build Move`) :`false` "QueryAndPhysics" :`true` "NoCollision" :!type "ECollisionEnabled Enum")))

(event `RefundAndDestroy (Server)`
  (params (PlayerController :type "Object Object Reference"))
  ;[1 1 1] Refund and Destroy / Move Building. Triggered when a player chooses to destroy a building.
  (`self.RefundAndDestroy` PlayerController)
  (`KismetSystemLibrary.Delay` 0.1)
  (`self.K2_DestroyActor`))

(event `/Game/SRPGE/Blueprints/Interfaces/BPI_Building.ResetBuildMaterial_BPI`
  ;[1 1 1] Refund and Destroy / Move Building. Triggered when a player chooses to destroy a building.
  (set `self.ResetMaterial` (not (`self.ResetMaterial`))))

(event `CollapseSupportCheck (Server)`
  (params (DestroyedActor :type "Actor Object Reference (by ref)") (Time :type "Float (single-precision)"))
  (bind _supportingactors (`self.SupportingActors`))
  (bind _groundactors (`self.GroundActors`))
  ;[1 1 1] Building Support/Collapse
  ;;[1 1 1] Enables a destroy timer and checks supporting actors for ground.
  (if (not (`self.CollapseChecked`))
    (set `self.CollapseTimer` Time)
    (bind _returnvalue (`KismetSystemLibrary.K2_SetTimerDelegate` (delegate `Destroy`) (`self.CollapseTimer`)))
    (set `self.DestroyTimer` _returnvalue)
    (if (`self.Debug - SupportMode`)
      (`PrimitiveComponent.SetMaterial` (`self.DebugSupportMesh`) 0 "/Game/SRPGE/Demo/Assets/Materials/Environment/MI_DebugTransparent_Red.MI_DebugTransparent_Red"))
    (set `self.CollapseChecked` true)
    (`KismetArrayLibrary.Array_Clear` (`self.GroundActors`))
    (`KismetArrayLibrary.Array_Clear` (`self.NonGroundActors`))
    (`KismetArrayLibrary.Array_RemoveItem` _supportingactors DestroyedActor)
    (bind (_array_element _array_index) (`/Game/SRPGE/Blueprints/Libraries/Lib_Macros.ForEachLoopNext` _supportingactors :!label _label_2)
      (:`Loop Body`
        (`/Engine/EditorBlueprintResources/StandardMacros.IsValid` _array_element
          (:`Is Valid`
            (if (`self.ActorHasTag` _array_element "IsOnGround")
              (`KismetArrayLibrary.Array_Add` (`self.GroundActors`) _array_element)
              (else
                (`KismetArrayLibrary.Array_Add` (`self.NonGroundActors`) _array_element)))
            (bind _asbp_building_master (cast `/Game/SRPGE/Blueprints/Actors/Building/BP_BuildingMaster` _array_element))
            (`self.CollapseSupportCheck (Server)` _asbp_building_master null (`self.CollapseTimer`))
            (`KismetSystemLibrary.DelayUntilNextTick`)
            (goto _label_2 :!via `NextLoop`))
          (:`Is Not Valid`
            (`KismetArrayLibrary.Array_Remove` _supportingactors _array_index))))
      (:`Complete`
        (for (_array_element_2 _array_index_2) _groundactors
          (`/Engine/EditorBlueprintResources/StandardMacros.IsValid` _array_element_2
            (:`Is Valid`
              (bind _asbp_building_master_2 (cast `/Game/SRPGE/Blueprints/Actors/Building/BP_BuildingMaster` _array_element_2))
              (if (`/Game/SRPGE/Blueprints/Actors/Building/BP_BuildingMaster.CollapseChecked` _asbp_building_master_2)
                (`self.StopCollapse (Server)` _asbp_building_master_2)))
            (:`Is Not Valid`
              (`KismetArrayLibrary.Array_Remove` _groundactors _array_index_2))))
        (if (`self.ActorHasTag` "IsOnGround")
          (`self.StopCollapse (Server)`))))))

(event `Destroy`
  ;[1 1 1] Building Support/Collapse
  ;;[1 1 1] Enables a destroy timer and checks supporting actors for ground.
  (set `self.CanTriggerCollapse` false)
  (`GameplayStatics.ApplyDamage` self (* (`self.Health`) -1.0) null self "/Engine/EngineDamageTypes/DmgTypeBP_Environmental.DmgTypeBP_Environmental_C"))

(event `StopCollapse (Server)`
  ;[1 1 1] Building Support/Collapse
  ;;[1 1 1] Stops the collapse and loops back through non-supported actors to ensure they also do not collapse.
  (`KismetSystemLibrary.Delay` 0.2)
  (if (`self.CollapseChecked`)
    (set `self.CollapseChecked` false)
    (`KismetSystemLibrary.K2_ClearAndInvalidateTimerHandle` (`self.DestroyTimer`))
    (for (_array_element _array_index) (`self.NonGroundActors`)
      (`/Engine/EditorBlueprintResources/StandardMacros.IsValid` _array_element
        (:`Is Valid`
          (bind _asbp_building_master (cast `/Game/SRPGE/Blueprints/Actors/Building/BP_BuildingMaster` _array_element))
          (`self.StopCollapse (Server)` _asbp_building_master))
        (:`Is Not Valid`
          (`KismetArrayLibrary.Array_Remove` (`self.NonGroundActors`) _array_index)))))
  (if (`self.Debug - SupportMode`)
    (`PrimitiveComponent.SetMaterial` (`self.DebugSupportMesh`) 0 (select `bool` (`self.ActorHasTag` "IsOnGround") :`false` "/Game/SRPGE/Demo/Assets/Materials/Environment/MI_DebugTransparent_Orange.MI_DebugTransparent_Orange" :`true` "/Game/SRPGE/Demo/Assets/Materials/Environment/MI_DebugTransparent_green.MI_DebugTransparent_green" :!type "MaterialInterface Object Reference"))))

(fn `ApplyDamage`
  (params (Damage :type "Float (double-precision)"))
  (returns (Destroyed :type Boolean))
  (set `self.Health` (+ (`self.Health`) Damage))
  (if (<= (`self.Health`) 0.0)
    (if (`KismetSystemLibrary.IsValidClass` (`self.Chaos Class`))
      (`self.DestroyBuilding (Server)` (`self.Chaos Class`)))
    (return true)))

(fn `CanBeDamaged_BPI`
  (params (RepName :type "GameplayTag Structure"))
  (returns (CanBeDamaged :type Boolean))
  (return (`self.CanBeDamaged`)))

(fn `CheckFaction_BPI`
  (params (RepName :type "GameplayTag Structure"))
  (returns (LevelName :type Name) (Hostile :type Boolean))
  (return "None" false))

(fn `CheckInteractable_BPI`
  (returns (CanInteract :type Boolean) (TriggerTime :type "Float (double-precision)"))
  (return (`self.CanRefund`) 0.4))

(fn `CheckIsAlive_BPI`
  (returns (Alive :type Boolean))
  (return false))

(fn `CheckSnapPoints`
  (params (Active :type Boolean) (Reset :type Boolean) (Destroy :type Boolean))
  (locals (LocalSnapPoint :type "/Game/SRPGE/Blueprints/Structures/Building/STR_BuildingSnaps Structure"))
  (bind _returnvalue (`self.K2_GetActorLocation`))
  (bind _active (`local.Active`))
  ;[1 1 1] Does a multi-sphere trace around the building to see what other buildings might be near that could have snap points. On Reset (Like when moving the building), wipes and resets the snap points. On destroy, doesn't bother touching self points.
  (if (`local.Reset`)
    (`KismetArrayLibrary.Array_Clear` (`self.SnapPoints`))
    (`self.SetupSnapPoints` (`.BuildSettings_9_D62D395642A8D48C0F6515B012605810` (break `/Game/SRPGE/Blueprints/Structures/Building/STR_BuildInfo` (`self.BuildInfo`))))
    (`self.SetSnaps (Server)`))
  (bind _outhits (`KismetSystemLibrary.SphereTraceMulti` _returnvalue _returnvalue (* (.y (`.BoxExtent` (`KismetMathLibrary.BreakBoxSphereBounds` (`StaticMesh.GetBounds` (`StaticMeshComponent.StaticMesh` (`self.StaticMesh`)))))) 1.4) "TraceTypeQuery4"))
  (for _array_element _outhits
    (if (not (`local.Destroy`))
      (bind (_bblockinghit _binitialoverlap _time _distance _location _impactpoint _normal _impactnormal _physmat _hitactor) (`GameplayStatics.BreakHitResult` _array_element))
      (message `/Game/SRPGE/Blueprints/Interfaces/BPI_Building.UpdateSnapIsActive_BPI` self (`self.K2_GetActorLocation` _hitactor) _active))
    (message `/Game/SRPGE/Blueprints/Interfaces/BPI_Building.UpdateSnapIsActive_BPI` _hitactor (`self.K2_GetActorLocation`) _active)))

(fn `CheckTool&Rarity_BPI`
  (returns (Required :type Boolean))
  (return false))

(fn `DestroyBuilding`
  ;[1 1 1] Destroys the Building
  (`ActorComponent.K2_DestroyComponent` (`self.StaticMesh`)))

(fn `GetBuildID_BPI`
  (returns (BuildID :type Name))
  (return (`self.BuildID`)))

(fn `GetBuildingManager_BPI`
  (returns (BuildingManager :type "/Game/SRPGE/Blueprints/Actors/Building/BP_BuildingManager Object Reference"))
  (return null))

(fn `GetBuildingManagerLevel_BPI`
  (returns (BuildingManagerLevel :type Integer))
  (return 0))

(fn `GetBuildingType_BPI`
  (returns (BuildingType :type "GameplayTag Structure"))
  (return))

(fn `GetContainerMaster_BPI`
  (returns (ContainerMaster :type "/Game/SRPGE/Blueprints/Actors/Building/BP_ContainerMaster Object Reference"))
  (return null))

(fn `GetDamagingActorName_BPI`
  (returns (Name :type Name))
  (return "None"))

(fn `GetFarmingMaster_BPI`
  (returns (`Farming Master` :type "/Game/SRPGE/Blueprints/Actors/Building/BP_FarmingMaster Object Reference"))
  (return null))

(fn `GetGameData_BPI`
  (returns (SaveGame :type "/Game/SRPGE/Blueprints/Game/SaveLoad/BP_Game_Save Object Reference"))
  (return null))

(fn `GetGameSettingsSaveData_BPI`
  (returns (AutoSave :type Boolean))
  (return false))

(fn `GetGUID_BPI`
  (returns (GUID :type "Guid Structure") (Type :type "/Game/SRPGE/Blueprints/Enumerators/E_SaveDataTypes Enum"))
  (bind _buildguid (`self.BuildGUID`))
  ;[1 1 1] Checks if the GUID is valid for save/load purposes
  (if (`KismetGuidLibrary.IsValid_Guid` _buildguid)
    (return _buildguid "NewEnumerator1")))

(fn `GetHarvestable_BPI`
  (returns (Harvestable :type "/Game/SRPGE/Blueprints/Actors/Interactables/Harvestables/BP_HarvestingMaster Object Reference"))
  (return null))

(fn `GetHitRequirements_BPI`
  (returns (ToolType :type "GameplayTagContainer Structure") (ToolRarity :type "GameplayTagContainer Structure"))
  (return (`self.Tool Type`) (`self.Tool Rarity`)))

(fn `GetInPowerZone_BPI`
  (returns (InZone :type Boolean))
  (return false))

(fn `GetInteractionTextUI_BPI`
  (returns (Text :type Text) (HideButton :type Boolean) (Offset :type "Vector Structure"))
  (return (select `bool` (`self.CanRefund`) :`true` "Destroy" :!type "Text") false (0.0 0.0 0.0)))

(fn `GetLookAtServer_BPI`
  (returns (LookAtServer :type Boolean))
  (return false))

(fn `GetPowerTower_BPI`
  (returns (PowerTower :type "/Game/SRPGE/Blueprints/Actors/Building/PowerSystem/BP_PowerTower Object Reference"))
  (return null))

(fn `GetResists_BPI`
  (returns (Resists :type "Map of GameplayTag Structure to Float (double-precision)"))
  (return))

(fn `GetSnapTransforms_BPI`
  (returns (SnapTransforms :type "Array of Transform Structure") (SnapTags :type "Array of Name"))
  (locals (LocalSnapTransforms :type "Array of Transform Structure") (LocalSnapTags :type "Array of Name"))
  ;[1 1 1] Returns valid snap transforms
  (for _array_element (`self.SnapPoints`)
    (bind (_transform _tag _active) (break `/Game/SRPGE/Blueprints/Structures/Building/STR_BuildingSnaps` _array_element))
    (if (not _active)
      (`KismetArrayLibrary.Array_Add` (`local.LocalSnapTransforms`) _transform)
      (`KismetArrayLibrary.Array_Add` (`local.LocalSnapTags`) _tag)))
  (return (`local.LocalSnapTransforms`) (`local.LocalSnapTags`)))

(fn `Init Building`
  (locals (LocalNewMesh :type "StaticMesh Object Reference") (LocalBuildTag :type Name) (LocalStaticMeshes :type "Array of StaticMeshComponent Object Reference"))
  (bind _returnvalue (`self.K2_GetActorLocation`))
  (bind ((`ChaosClass_50_04C23AF446F2BEBDAB9426B2DB459BAA` _chaosclass) (`BuildSettings_9_D62D395642A8D48C0F6515B012605810` _buildsettings) (`RequiresBuildManager_61_BACE3A1F4161E45E0F1062B9E95319FE` _requiresbuildmanager) (`IsBuildSurface_64_5D41EF0447847E61236239B42F318DC4` _isbuildsurface)) (break `/Game/SRPGE/Blueprints/Structures/Building/STR_BuildInfo` (`self.BuildInfo`)))
  ;[1 1 1] Using the Build Info, checks defined snap points and calulates their position based on the placement position/rotation of the new build. Stores the transforms for snapping.
  (bind _returnvalue_2 (`|GetDataTableRow` "/Game/SRPGE/Blueprints/DataTables/DT_Buildings.DT_Buildings" (`self.BuildID`))
    (:`then`
      (set `self.BuildInfo` _returnvalue_2)
      (`self.Load&SetMesh`)
      (set `self.Chaos Class` _chaosclass)
      (set `self.Requires Build Manager` _requiresbuildmanager)
      (if _isbuildsurface
        (`KismetArrayLibrary.Array_Add` (`ActorComponent.ComponentTags` (`self.StaticMesh`)) "BuildSurface"))
      (`self.SetupSnapPoints` _buildsettings)
      (bind (_outhits _returnvalue_3) (`KismetSystemLibrary.LineTraceMulti` (+ _returnvalue (0.0 0.0 150.0)) (+ _returnvalue (0.0 0.0 -150.0)) "TraceTypeQuery1"))
      (if _returnvalue_3
        (for _array_element _outhits
          (if (`self.ActorHasTag` (`.HitActor` (`GameplayStatics.BreakHitResult` _array_element)) "Ground")
            (`KismetArrayLibrary.Array_Add` (`self.Tags`) "IsOnGround")
            (break)))))))

(fn `LoadObjectData_BPI`
  (params (SaveGame :type "/Game/SRPGE/Blueprints/Game/SaveLoad/BP_Game_Save Object Reference"))
  (returns (Success :type Boolean))
  (return false))

(fn `OnRep_Build Mesh`
  ;[1 1 1] Must be set via a rep notify to ensure newly joining clients get the update
  (`StaticMeshComponent.SetStaticMesh` (`self.StaticMesh`) (`self.Build Mesh`))
  (set `self.BaseMats` (`MeshComponent.GetMaterials` (`self.StaticMesh`))))

(fn `OnRep_BuildingManager`)

(fn `OnRep_ResetMaterial`
  (for (_array_element _array_index) (`self.BaseMats`)
    (`self.SetMaterial` _array_index _array_element))
  (set `self.Build Move` false))

(fn `RefundAndDestroy`
  (params (PlayerController :type "Object Object Reference"))
  ;[1 1 1] Gets the building requirements for this building and returns them to the player controller that destroyed the building. Then destroys it.
  (for _array_element (`.BuildCost_42_D3F3FAA24C96F91BC62222B297F27008` (break `/Game/SRPGE/Blueprints/Structures/Building/STR_BuildInfo` (`self.BuildInfo`)))
    (bind ((`Item_2_587C73524DD029F60D1D5B8EBC2BDD23` _item) (`Quantity_5_B4B993734135FE49DBC79D923FBFDCB1` _quantity)) (break `/Game/SRPGE/Blueprints/Structures/Inventory/STR_ItemList` _array_element))
    (bind _row (`/Game/SRPGE/Blueprints/Libraries/Lib_Functions.Get Item DT Row` _item))
    (bind _structout (setmembers `/Game/SRPGE/Blueprints/Structures/Inventory/STR_ItemValues` :`StructRef` (`.CurrentItemValues_68_EAF0DA8A4E892330842804B79249E216` (break `/Game/SRPGE/Blueprints/Structures/Inventory/STR_ItemData` _row)) :`StackCount` _quantity))
    (bind _structout_2 (setmembers `/Game/SRPGE/Blueprints/Structures/Inventory/STR_ItemData` :`StructRef` _row :`CurrentItemValues` _structout))
    (bind (_success _remainingitems) (message `/Game/SRPGE/Blueprints/Interfaces/BPI_PlayerController.TryAddItem_BPI` (`local.PlayerController`) _structout_2))
    (if (not _success)
      (message `/Game/SRPGE/Blueprints/Interfaces/BPI_PlayerController.SpawnItemAtLoc_BPI` (`local.PlayerController`) _item _remainingitems)))
  (`self.DestroyBuilding (Server)` (`self.Chaos Class`))
  (`self.CheckSnapPoints` false false true))

(fn `SaveObjectData_BPI`
  (params (SaveGame :type "/Game/SRPGE/Blueprints/Game/SaveLoad/BP_Game_Save Object Reference"))
  (returns (Success :type Boolean))
  ;[1 1 1] Sets the save data for the building master
  (`KismetArrayLibrary.Array_Add` (`/Game/SRPGE/Blueprints/Game/SaveLoad/BP_Game_Save.BuildingMasters` SaveGame) (make `/Game/SRPGE/Blueprints/Structures/SaveLoad/STR_SaveGame_BuildingMaster` :`BuildGUID` (`self.BuildGUID`) :`BuildingClass` (`GameplayStatics.GetObjectClass` self) :`BuildTransform` (`self.GetTransform`) :`BuildID` (`self.BuildID`) :`PlayerBuild` (`self.Player Build`)))
  (return true))

(fn `SetMaterial`
  (params (ElementIndex :type Integer) (Material :type "MaterialInterface Object Reference"))
  (for _array_element (`self.K2_GetComponentsByClass` "/Script/Engine.PrimitiveComponent")
    (`PrimitiveComponent.SetMaterial` _array_element ElementIndex Material)))

(fn `SetSnapUsed`
  (params (SnapLocation :type "Vector Structure") (Active :type Boolean))
  (locals (LocalSnapPoint :type "/Game/SRPGE/Blueprints/Structures/Building/STR_BuildingSnaps Structure"))
  ;[1 1 1] Checks incoming location against snap points, updating the active status if found.
  (for (_array_element _array_index) (`self.SnapPoints`)
    (set `local.LocalSnapPoint` _array_element)
    (if (== SnapLocation (.location (`.Transform_2_1E89787543EDEBEE4F23E789018B3A42` (break `/Game/SRPGE/Blueprints/Structures/Building/STR_BuildingSnaps` (`local.LocalSnapPoint`)))) :`ErrorTolerance` 25.0)
      (bind _structout (setmembers `/Game/SRPGE/Blueprints/Structures/Building/STR_BuildingSnaps` :`StructRef` (`local.LocalSnapPoint`) :`Active` (`local.Active`)))
      (`KismetArrayLibrary.Array_Set` (`self.SnapPoints`) _array_index _structout)))
  (`self.SetSnaps (Server)`))

(fn `SetupSnapPoints`
  (params (Array :type "Array of /Game/SRPGE/Blueprints/Structures/Building/STR_BuildSettings Structure"))
  (locals (LocalBuildTag :type Name))
  ;[1 1 1] Sets up snap points based on data table.
  (for _array_element Array
    (bind (_mesh _buildingtag _positionsettings _previewcolor) (break `/Game/SRPGE/Blueprints/Structures/Building/STR_BuildSettings` _array_element))
    (set `local.LocalBuildTag` _buildingtag)
    (for _array_element_2 _positionsettings
      (bind (_position _rotator) (break `/Game/SRPGE/Blueprints/Structures/Building/STR_BuildPos` _array_element_2))
      (bind _returnvalue (`KismetMathLibrary.ComposeTransforms` (`KismetMathLibrary.MakeTransform` _position (`KismetMathLibrary.MakeRotator` (.roll _rotator) (.pitch _rotator) (.yaw _rotator))) (`self.GetTransform`)))
      (`KismetArrayLibrary.Array_Add` (`self.SnapPoints`) (make `/Game/SRPGE/Blueprints/Structures/Building/STR_BuildingSnaps` _returnvalue (`local.LocalBuildTag`)))
      (if (`self.Debug - SetupMode`)
        (bind _returnvalue_2 (`AddComponent|NODE_AddStaticMeshComponent-4` :`RelativeTransform` _returnvalue))
        (`StaticMeshComponent.SetStaticMesh` _returnvalue_2 _mesh)
        (bind _returnvalue_3 (`KismetMaterialLibrary.CreateDynamicMaterialInstance` "/Game/SRPGE/Demo/Assets/Meshes/Buildings/Materials/MI_PreviewColor_Inst.MI_PreviewColor_Inst"))
        (`PrimitiveComponent.SetMaterial` _returnvalue_2 0 _returnvalue_3)
        (`MaterialInstanceDynamic.SetVectorParameterValue` _returnvalue_3 "Color" _previewcolor))))
  (`self.SetSnaps (Server)`))

(fn `ShouldOutline_BPI`
  (returns (Outline :type Boolean) (CustomDepth :type Integer))
  (return (`self.CanRefund`) 1))

(fn `UserConstructionScript`
  (locals (LocalNewMesh :type "StaticMesh Object Reference") (LocalBuildTag :type Name) (LocalStaticMeshes :type "Array of StaticMeshComponent Object Reference"))
  ;[1 1 1] Used for setting up new buildings
  (set `self.BuildGUID` (`self.ActorGuid`))
  (if (`self.Debug - SetupMode`)
    (`self.Init Building`)))