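; A chest variant of a buildable container that animates its lid and plays a sound as players start and stop using it.
; Server add/remove user events extend the parent, then pass the user count to a multicast that opens the lid for the first user and closes it for the last.
; Opening also jostles the mesh, then restores the location cached on interaction; a lock-shake timeline is left unconnected.
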(event `/Game/SRPGE/Blueprints/Interfaces/BPI_Interaction.TriggerInteraction_BPI`
  (params (PlayerController :type "Controller Object Reference") (PlayerCharacter :type "/Game/SRPGE/Blueprints/Player/BP_PlayerCharacter Object Reference") (BuildRefund :type Boolean))
  (set `self.Location` (`SceneComponent.K2_GetComponentLocation` (`self.StaticMesh`)))
  (`parent.TriggerInteraction_BPI` PlayerController PlayerCharacter BuildRefund))

(event `ChestEffect (MC)`
  (params (Condition :type Boolean) (Length :type Integer))
  ;[1 1 1] Plays opening/closing effecting. Only plays when the first person opens the chest or the last person closes it.
  (if (and Condition (== Length 1))
    (bind (_direction _lidrotation _meshlocation _meshrotation) (`Timeline|OpenTimeline` :!via `PlayFromStart`)
      (:`Update`
        (`SceneComponent.K2_SetRelativeRotation` (`self.Lid`) (`KismetMathLibrary.MakeRotator` (.x _lidrotation) (.y _lidrotation) (.z _lidrotation)) false false)
        (`SceneComponent.K2_AddRelativeLocation` (`self.StaticMesh`) _meshlocation false false)
        (`SceneComponent.K2_SetRelativeRotation` (`self.StaticMesh`) (`KismetMathLibrary.MakeRotator` _meshrotation) false false))
      (:`Finished`
        (`SceneComponent.K2_SetWorldLocation` (`self.StaticMesh`) (`self.Location`) false false)))
    (elif (and (== Length 0) (not Condition))
      (bind (_direction_2 _lidrotation_2) (`Timeline|CloseTimeline` :!via `PlayFromStart`)
        (:`Update`
          (`SceneComponent.K2_SetRelativeRotation` (`self.Lid`) (`KismetMathLibrary.MakeRotator` (.x _lidrotation_2) (.y _lidrotation_2) (.z _lidrotation_2)) false false))))))

(event `self.AddUsingPlayer (Server)`
  (params (PlayerController :type "Controller Object Reference"))
  (`parent.AddUsingPlayer (Server)` PlayerController)
  (`self.ChestEffect (MC)` true (`KismetArrayLibrary.Array_Length` (`self.UsingPlayers`)))
  (`GameplayStatics.PlaySoundAtLocation` "/Game/SRPGE/Demo/Assets/Audio/SFX/SW_Chest.SW_Chest" (`self.K2_GetActorLocation`) (struct) 1.0 1.0 0.0 null null null null))

(event `self.RemoveUsingPlayer (Server)`
  (params (PlayerController :type "Controller Object Reference (by ref)"))
  (`parent.RemoveUsingPlayer (Server)` PlayerController)
  (`self.ChestEffect (MC)` false (`KismetArrayLibrary.Array_Length` (`self.UsingPlayers`)))
  (`GameplayStatics.PlaySoundAtLocation` "/Game/SRPGE/Demo/Assets/Audio/SFX/SW_Chest.SW_Chest" (`self.K2_GetActorLocation`) (struct) 1.0 1.0 0.0 null null null null))

(event `self.Load&SetMesh`
  (set `self.Build Mesh` "/Game/SRPGE/Demo/Assets/Meshes/New/SM_chest_gold.SM_chest_gold"))

(fn `UserConstructionScript`
  (`parent.UserConstructionScript`))