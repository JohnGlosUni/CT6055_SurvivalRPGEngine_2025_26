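; Preview character actor for the character creator, exposing events to swap the skeletal mesh, play montages and change tint color.
; BeginPlay creates Manny and Quinn dynamic materials, with only Manny's applied to the mesh; color changes set Tint on both from an enum.
; CreateDynamicRT builds a render target and material at runtime, giving each client its own preview instance and returning the material to the UI.
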(event `PlayAnimation`
  (params (AnimMontage :type "AnimMontage Object Reference"))
  (`self.PlayAnimMontage` AnimMontage))

(event `self.ReceiveBeginPlay`
  ;[1 1 1] Sets starting Mesh and creates both dynamic materials
  (bind _returnvalue (`PrimitiveComponent.CreateDynamicMaterialInstance` (`self.Mesh`) 1 "/Game/SRPGE/Demo/Characters/Mannequins/Materials/Instances/Manny/MI_Manny_01.MI_Manny_01" "None"))
  (set `self.Mat` _returnvalue)
  (bind _returnvalue_2 (`KismetMaterialLibrary.CreateDynamicMaterialInstance` "/Game/SRPGE/Demo/Characters/Mannequins/Materials/Instances/Quinn/MI_Quinn_01.MI_Quinn_01"))
  (set `self.Mat_2` _returnvalue_2))

(event `UpdateColor`
  (params (Color :type "/Game/SRPGE/Blueprints/Enumerators/E_Colors Enum" :default "NewEnumerator0"))
  ;[1 1 1] Updates color
  (`MaterialInstanceDynamic.SetVectorParameterValue` (`self.Mat`) "Tint" (select `/Game/SRPGE/Blueprints/Enumerators/E_Colors` Color :`NewEnumerator0` (struct :`R` 1.0 :`B` 0.017848 :`A` 1.0) :`NewEnumerator2` (struct :`R` 0.002067 :`G` 1.0 :`A` 1.0) :`NewEnumerator3` (struct :`R` 1.0 :`G` 1.0 :`B` 1.0 :`A` 1.0) :`NewEnumerator4` (struct :`G` 0.242042 :`B` 1.0 :`A` 1.0) :!type "LinearColor Structure"))
  (`MaterialInstanceDynamic.SetVectorParameterValue` (`self.Mat_2`) "Tint" (select `/Game/SRPGE/Blueprints/Enumerators/E_Colors` Color :`NewEnumerator0` (struct :`R` 1.0 :`B` 0.017848 :`A` 1.0) :`NewEnumerator2` (struct :`R` 0.002067 :`G` 1.0 :`A` 1.0) :`NewEnumerator3` (struct :`R` 1.0 :`G` 1.0 :`B` 1.0 :`A` 1.0) :`NewEnumerator4` (struct :`G` 0.242042 :`B` 1.0 :`A` 1.0) :!type "LinearColor Structure")))

(event `UpdateMesh`
  (params (NewMesh :type "SkeletalMesh Object Reference"))
  ;[1 1 1] Updates Mesh and Material
  (`SkeletalMeshComponent.SetSkeletalMeshAsset` (`self.Mesh`) NewMesh))

(fn `Create Dynamic RT`
  (returns (ReturnValue :type "MaterialInstanceDynamic Object Reference"))
  (locals (LocalMaterial :type "MaterialInstanceDynamic Object Reference"))
  ;[1 1 1] Creates a dynamic render target to ensure each client has it's own unique instance. Returns the material to the UI.
  (bind _returnvalue (`KismetRenderingLibrary.CreateRenderTarget2D` 1024 1024))
  (bind _returnvalue_2 (`KismetMaterialLibrary.CreateDynamicMaterialInstance` "/Game/SRPGE/Blueprints/UserInterface/HUD/Overlays/RT_CharacterCreator_Mat.RT_CharacterCreator_Mat"))
  (set `local.LocalMaterial` _returnvalue_2)
  (set `SceneCaptureComponent2D.TextureTarget` _returnvalue (`self.RenderTarget`))
  (`MaterialInstanceDynamic.SetTextureParameterValue` (`local.LocalMaterial`) "RenderTarget" _returnvalue)
  (return (`local.LocalMaterial`)))

(fn `UserConstructionScript`)