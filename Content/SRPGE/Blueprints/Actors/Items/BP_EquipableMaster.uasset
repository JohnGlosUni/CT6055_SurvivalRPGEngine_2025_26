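; Base actor for equipable items held in a character's hands, exposing itself through an equipable interface call.
; On BeginPlay it sets Ammo from the item's extension data.
; Triggering it plays the default character montage on the player via an interface message, leaving further functionality to notifies in the montage.
; Save and load interface functions are overridden to only return true, so held items skip persistence.
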(event `self.ReceiveBeginPlay`
  (bind (_value _returnvalue) (`BlueprintMapLibrary.Map_Find` (`.Extensions_34_2DD9433F443CFC611B3F258C9DD5FD4F` (break `/Game/SRPGE/Blueprints/Structures/Inventory/STR_ItemData` (`self.Item`))) "Ammo"))
  ;[1 1 1] Sets Ammo type from the item info
  (if _returnvalue
    (set `self.Ammo` _value)))

(event `/Game/SRPGE/Blueprints/Interfaces/BPI_Equipable.TriggerEquipable_BPI`
  (params (StateRef :type "/Game/SRPGE/Blueprints/Player/BP_PlayerState Object Reference") (PlayerRef :type "/Game/SRPGE/Blueprints/Player/BP_PlayerCharacter Object Reference") (ControllerRef :type "PlayerController Object Reference"))
  (bind (_value _returnvalue) (`BlueprintMapLibrary.Map_Find` (`.CharacterMontage_26_43D3415F4C9D3C192DDFFEA357F7D45A` (break `/Game/SRPGE/Blueprints/Structures/Inventory/STR_Equipable` (`self.EquipableInfo`))) "Default"))
  ;[1 1 1] Plays equipable montage. Notfies for additional functionality are in the Montage itself
  (if _returnvalue
    (message `/Game/SRPGE/Blueprints/Interfaces/BPI_PlayerCharacter.PlayAnimMontage_BPI` PlayerRef _value)))

(fn `GetEquipable_BPI`
  (returns (Equipable :type "/Game/SRPGE/Blueprints/Actors/Items/BP_EquipableMaster Object Reference"))
  (return self))

(fn `LoadObjectData_BPI`
  (params (SaveGame :type "/Game/SRPGE/Blueprints/Game/SaveLoad/BP_Game_Save Object Reference"))
  (returns (Success :type Boolean))
  ;[1 1 1] Overriden to ensure equipped items in hands aren't saving/loading
  (return true))

(fn `SaveObjectData_BPI`
  (params (SaveGame :type "/Game/SRPGE/Blueprints/Game/SaveLoad/BP_Game_Save Object Reference"))
  (returns (Success :type Boolean))
  ;[1 1 1] Overriden to ensure equipped items in hands aren't saving/loading
  (return true))

(fn `UserConstructionScript`
  (`parent.UserConstructionScript`))