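; Base world item actor for placed or dropped pickups, collected by interaction or, for auto-collect drops, by flying to the player after a short delay.
; InitItem builds item data from a data table row and loads meshes, async when packaged and blocking otherwise, applied through OnReps.
; Rarity drives outline stencil and Niagara color.
; Failed inventory adds keep the remaining stack, and state is saved with a GUID.
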(event `self.ReceiveBeginPlay`
  ;[1 1 1] Refreshes item data from the data table. Updates in world items that aren't part of the save file yet.
  (`self.SetRarity`)
  (if (`self.Dropped`)
    (`PrimitiveComponent.SetCollisionResponseToChannel` (`self.StaticMesh`) "ECC_GameTraceChannel1" "ECR_Block")
    (if (`self.AutoCollect`)
      ;[1 1 1] Ensures the spheres can't be picked up instantly. Default Sphere Radius = 0
      (bind _returnvalue (`KismetSystemLibrary.K2_SetTimerDelegate` (delegate `EnablePickup`) 0.8))
      (set `self.PickupTimer` _returnvalue)
      (else
        (`ActorComponent.K2_DestroyComponent` (`self.Sphere`) :!label _label)))
    (else
      (goto _label))))

(event `EnablePickup`
  ;[1 1 1] Ensures the spheres can't be picked up instantly. Default Sphere Radius = 0
  (set `self.PickupEnabled` true)
  (`KismetSystemLibrary.K2_ClearAndInvalidateTimerHandle` (`self.PickupTimer`))
  (`SphereComponent.SetSphereRadius` (`self.Sphere`) 300.0 true))

(event `self.Sphere.OnComponentBeginOverlap`
  (params (OverlappedComponent :type "PrimitiveComponent Object Reference") (OtherActor :type "Actor Object Reference") (OtherComp :type "PrimitiveComponent Object Reference") (OtherBodyIndex :type Integer) (bFromSweep :type Boolean) (SweepResult :type "HitResult Structure (by ref)"))
  (bind _staticmesh (`self.StaticMesh`))
  (bind _staticmesh_2 (`self.StaticMesh`))
  (bind _item (`self.Item`))
  ;[1 1 1] Auto Collection
  ;;[1 1 1] Ensures pickup is enabled and the target is not already moving. Gets the collection point from the character. Triggers on both begin and end as the user may be in the sphere when pickup is enabled
  (set `self.Other Actor` OtherActor)
  (if (and (`self.PickupEnabled`) (not (`self.Moving`)) (`KismetSystemLibrary.IsValid` (`self.Other Actor`))) :!label _label_2
    (bind _player (message `/Game/SRPGE/Blueprints/Interfaces/BPI_PlayerCharacter.GetPlayerCharacter_BPI` (`self.Other Actor`)))
    (`/Engine/EditorBlueprintResources/StandardMacros.IsValid` _player
      (:`Is Valid`
        (set `self.CollectionTarget` (`/Game/SRPGE/Blueprints/Player/BP_PlayerCharacter.CollectionPoint` _player))
        (set `self.Moving` true)
        (`|ExecutionSequence`
          (:`then_0`
            ;;[1 1 1] Disables Physics
            (`PrimitiveComponent.SetCollisionResponseToChannel` (`self.StaticMesh`) "ECC_Pawn" "ECR_Ignore")
            (`PrimitiveComponent.SetCollisionEnabled` (`self.Sphere`) "NoCollision"))
          (:`then_1`
            (bind (_direction _movetrack) (`Timeline|Timeline` :!via `PlayFromStart`)
              (:`Update`
                ;;[1 1 1] Moves mesh towards character, lerped from 0 --> 1 via a timeline
                (`/Engine/EditorBlueprintResources/StandardMacros.IsValid` _staticmesh_2
                  (:`Is Valid`
                    (`SceneComponent.K2_SetWorldLocation` _staticmesh_2 (`KismetMathLibrary.VLerp` (`SceneComponent.K2_GetComponentLocation` _staticmesh_2) (`SceneComponent.K2_GetComponentLocation` (`self.CollectionTarget`)) _movetrack) false true))))
              (:`Finished`
                ;;[1 1 1] Adds items to inventory and destroys the actor
                (bind (_success _remainingitems) (message `/Game/SRPGE/Blueprints/Interfaces/BPI_PlayerController.TryAddItem_BPI` (`Pawn.GetController` _player) _item))
                (if _success
                  (`self.K2_DestroyActor`)
                  (else
                    (bind _structout (setmembers `/Game/SRPGE/Blueprints/Structures/Inventory/STR_ItemValues` :`StructRef` (`.CurrentItemValues_68_EAF0DA8A4E892330842804B79249E216` (break `/Game/SRPGE/Blueprints/Structures/Inventory/STR_ItemData` _item)) :`StackCount` _remainingitems))
                    (bind _structout_2 (setmembers `/Game/SRPGE/Blueprints/Structures/Inventory/STR_ItemData` :`StructRef` _item :`CurrentItemValues` _structout))
                    (set `self.Item` _structout_2)
                    (`PrimitiveComponent.SetSimulatePhysics` _staticmesh true)
                    (`PrimitiveComponent.SetCollisionEnabled` _staticmesh "QueryAndPhysics")))))))))))

(event `self.Sphere.OnComponentEndOverlap`
  (params (OverlappedComponent :type "PrimitiveComponent Object Reference") (OtherActor :type "Actor Object Reference") (OtherComp :type "PrimitiveComponent Object Reference") (OtherBodyIndex :type Integer))
  ;[1 1 1] Auto Collection
  ;;[1 1 1] Ensures pickup is enabled and the target is not already moving. Gets the collection point from the character. Triggers on both begin and end as the user may be in the sphere when pickup is enabled
  (set `self.Other Actor` OtherActor)
  (goto _label_2))

(event `/Game/SRPGE/Blueprints/Interfaces/BPI_Interaction.TriggerInteraction_BPI`
  (params (PlayerController :type "Controller Object Reference") (PlayerCharacter :type "/Game/SRPGE/Blueprints/Player/BP_PlayerCharacter Object Reference") (BuildRefund :type Boolean))
  (bind _item (`self.Item`))
  ;[1 1 1] Tries to add the item to the players inventory. Updates stack count if not successful (As some items may have been added)
  (bind (_success _remainingitems) (message `/Game/SRPGE/Blueprints/Interfaces/BPI_PlayerController.TryAddItem_BPI` PlayerController _item))
  (if (`self.Debug`)
    _
    (elif _success
      (`self.K2_DestroyActor`)
      (else
        (bind _structout (setmembers `/Game/SRPGE/Blueprints/Structures/Inventory/STR_ItemValues` :`StructRef` (`.CurrentItemValues_68_EAF0DA8A4E892330842804B79249E216` (break `/Game/SRPGE/Blueprints/Structures/Inventory/STR_ItemData` _item)) :`StackCount` _remainingitems))
        (bind _structout_2 (setmembers `/Game/SRPGE/Blueprints/Structures/Inventory/STR_ItemData` :`StructRef` _item :`CurrentItemValues` _structout))
        (set `self.Item` _structout_2)))))

(event `/Game/SRPGE/Blueprints/Interfaces/BPI_Interaction.SetItemData_BPI`
  (params (ItemHandle :type "DataTableRowHandle Structure") (StackCount :type Integer) (AmmoCount :type Integer) (Durability :type "Float (double-precision)") (Decay :type "Float (double-precision)"))
  ;[1 1 1] Sets item data when spawning or loading the item
  (`self.Set Item Data (Server)` ItemHandle StackCount AmmoCount Durability Decay)
  (`self.Set Item Data (Client)`))

(event `Set Item Data (Server)`
  (params (ItemHandle :type "DataTableRowHandle Structure") (StackCount :type Integer) (AmmoCount :type Integer) (Durability :type "Float (double-precision)") (Decay :type "Float (double-precision)"))
  ;[1 1 1] Sets item data when spawning or loading the item
  (`self.InitItem` ItemHandle StackCount AmmoCount Durability Decay))

(event `Set Item Data (Client)`
  ;[1 1 1] Sets item data when spawning or loading the item
  (`self.SetRarity`))

(event `/Game/SRPGE/Blueprints/Interfaces/BPI_SaveLoad_Game.SetItemSaveData_BPI`
  (params (ItemData :type "/Game/SRPGE/Blueprints/Structures/SaveLoad/STR_SaveGame_ItemMaster Structure"))
  (bind ((`ItemID_17_B7F3672D4761DE87B2DB6DBB286683B9` _itemid) (`StackCount_16_C58804F14488111BFDF421B3E320EA91` _stackcount) (`AmmoCount_15_393972414A4DC69FA3E82CA9A32DB3D9` _ammocount) (`Durability_14_4F7AEB314111A72F05C21F8CD7AFFC93` _durability) (`Decay_13_55C464DF417FE4866830A897FEF7E970` _decay)) (break `/Game/SRPGE/Blueprints/Structures/SaveLoad/STR_SaveGame_ItemMaster` ItemData))
  ;[1 1 1] Sets item data when spawning or loading the item
  (`self.Set Item Data (Server)` _itemid _stackcount _ammocount _durability _decay))

(event `Load&SetMesh`
  (bind ((`EquipableInfo_96_27EC872442B9F73A62282794B4A2BC78` _equipableinfo) (`StaticMeshes_90_EC20606B4A62F2B6CDFA35A728B93D9F` _staticmeshes) (`SkeletalMeshes_91_E15C7D244C82EB1710A93397066E9995` _skeletalmeshes)) (break `/Game/SRPGE/Blueprints/Structures/Inventory/STR_ItemData` (`self.Item`)))
  (bind _value (`BlueprintMapLibrary.Map_Find` _skeletalmeshes "Default"))
  (bind _value_2 (`BlueprintMapLibrary.Map_Find` _staticmeshes "Default"))
  ;[1 1 1] Loads the item mesh based on the incoming item data. If the mesh is a skeletal Mesh, adds a skeletal mesh component and hides the static mesh.
  (`|ExecutionSequence`
    (:`then_0`
      (if (`KismetSystemLibrary.IsValidSoftObjectReference` _value_2)
        (bind _object (`|LoadAsset` _value_2)
          (:`Completed`
            (bind _asstatic_mesh (cast `StaticMesh` _object))
            (set `self.DefaultMesh` _asstatic_mesh)))))
    (:`then_1`
      (if (`KismetSystemLibrary.IsValidSoftObjectReference` _value)
        (bind _object_2 (`|LoadAsset` _value)
          (:`Completed`
            (bind _asskeletal_mesh (cast `SkeletalMesh` _object_2))
            (bind _returnvalue (`AddComponent|NODE_AddSkeletalMeshComponent-0`))
            (set `self.SkeletalMesh` _returnvalue)
            (set `self.DefaultSkeletalMesh` _asskeletal_mesh)))))))

(event `Editor - Load&SetMesh`
  (bind ((`EquipableInfo_96_27EC872442B9F73A62282794B4A2BC78` _equipableinfo) (`StaticMeshes_90_EC20606B4A62F2B6CDFA35A728B93D9F` _staticmeshes) (`SkeletalMeshes_91_E15C7D244C82EB1710A93397066E9995` _skeletalmeshes)) (break `/Game/SRPGE/Blueprints/Structures/Inventory/STR_ItemData` (`self.Item`)))
  (bind _value (`BlueprintMapLibrary.Map_Find` _staticmeshes "Default"))
  (bind _value_2 (`BlueprintMapLibrary.Map_Find` _skeletalmeshes "Default"))
  ;[1 1 1] Loads the item mesh based on the incoming item data. If the mesh is a skeletal Mesh, adds a skeletal mesh component and hides the static mesh.
  (`|ExecutionSequence`
    (:`then_0`
      (if (`KismetSystemLibrary.IsValidSoftObjectReference` _value)
        (bind _returnvalue (`KismetSystemLibrary.LoadAsset_Blocking` _value))
        (bind _asstatic_mesh (cast `StaticMesh` _returnvalue))
        (set `self.DefaultMesh` _asstatic_mesh)))
    (:`then_1`
      (if (`KismetSystemLibrary.IsValidSoftObjectReference` _value_2)
        (bind _returnvalue_2 (`KismetSystemLibrary.LoadAsset_Blocking` _value_2))
        (bind _asskeletal_mesh (cast `SkeletalMesh` _returnvalue_2))
        (bind _returnvalue_3 (`AddComponent|NODE_AddSkeletalMeshComponent-1`))
        (set `self.SkeletalMesh` _returnvalue_3)
        (set `self.DefaultSkeletalMesh` _asskeletal_mesh)))))

(fn `CheckInteractable_BPI`
  (returns (CanInteract :type Boolean) (TriggerTime :type "Float (double-precision)"))
  ;[1 1 1] Can only be interacted with if item is valid
  (return (`/Game/SRPGE/Blueprints/Libraries/Lib_Functions.ItemIsValid` (`self.Item`)) 0.0))

(fn `GetGameData_BPI`
  (returns (SaveGame :type "/Game/SRPGE/Blueprints/Game/SaveLoad/BP_Game_Save Object Reference"))
  (return null))

(fn `GetGameSettingsSaveData_BPI`
  (returns (AutoSave :type Boolean))
  (return false))

(fn `GetGUID_BPI`
  (returns (GUID :type "Guid Structure") (Type :type "/Game/SRPGE/Blueprints/Enumerators/E_SaveDataTypes Enum"))
  (return (`self.ItemGUID`) "NewEnumerator0"))

(fn `GetHarvestable_BPI`
  (returns (Harvestable :type "/Game/SRPGE/Blueprints/Actors/Interactables/Harvestables/BP_HarvestingMaster Object Reference"))
  (return null))

(fn `GetHitRequirements_BPI`
  (returns (ToolType :type "GameplayTagContainer Structure") (ToolRarity :type "GameplayTagContainer Structure"))
  (return))

(fn `GetInteractionTextUI_BPI`
  (returns (Text :type Text) (HideButton :type Boolean) (Offset :type "Vector Structure"))
  (bind ((`Name_18_C4509765484F9DEB5F04E0AF6E49160B` _name) (`CurrentItemValues_68_EAF0DA8A4E892330842804B79249E216` _currentitemvalues)) (break `/Game/SRPGE/Blueprints/Structures/Inventory/STR_ItemData` (`self.Item`)))
  (return (`|FormatText` "Pick Up: {x} x{y}" _name (`.StackCount_10_03F2C0784ACF404210724DAFD1673A9C` (break `/Game/SRPGE/Blueprints/Structures/Inventory/STR_ItemValues` _currentitemvalues))) false (0.0 0.0 0.0)))

(fn `GetLookAtServer_BPI`
  (returns (LookAtServer :type Boolean))
  (return false))

(fn `InitItem`
  (params (ItemHandleRow :type "DataTableRowHandle Structure") (StackCount :type Integer) (AmmoCount :type Integer) (Durability :type "Float (double-precision)") (Decay :type "Float (double-precision)"))
  ;[1 1 1] Sets up item based on incoming data. Data is comes from the world (if placed in editor) or from a spawn such as item drop.
  (set `self.ItemID` ItemHandleRow)
  (bind _row (`/Game/SRPGE/Blueprints/Libraries/Lib_Functions.Get Item DT Row` (`self.ItemID`)))
  (bind _structout (setmembers `/Game/SRPGE/Blueprints/Structures/Inventory/STR_ItemData` :`StructRef` _row :`CurrentItemValues` (make `/Game/SRPGE/Blueprints/Structures/Inventory/STR_ItemValues` StackCount AmmoCount Durability Decay)))
  (set `self.Item` _structout)
  (set `self.EquipableInfo` (`.EquipableInfo_96_27EC872442B9F73A62282794B4A2BC78` (break `/Game/SRPGE/Blueprints/Structures/Inventory/STR_ItemData` (`self.Item`))))
  (if (`KismetSystemLibrary.IsPackagedForDistribution`)
    (`self.Load&SetMesh`)
    (else
      (`self.Editor - Load&SetMesh`))))

(fn `LoadObjectData_BPI`
  (params (SaveGame :type "/Game/SRPGE/Blueprints/Game/SaveLoad/BP_Game_Save Object Reference"))
  (returns (Success :type Boolean))
  (return false))

(fn `OnRep_DefaultMesh`
  (bind _staticmesh (`self.StaticMesh`))
  (bind _staticmesh_2 (`self.StaticMesh`))
  ;[1 1 1] Sets the mesh for all clients. If the item was dropped, gives it collision so it can be picked up.
  (`StaticMeshComponent.SetStaticMesh` _staticmesh (`self.DefaultMesh`))
  (`SceneComponent.SetRelativeScale3D` _staticmesh (`.DropItemSizing_94_B64DE2734B2137603489228783672990` (break `/Game/SRPGE/Blueprints/Structures/Inventory/STR_ItemData` (`self.Item`))))
  (if (`self.Dropped`)
    (`PrimitiveComponent.SetCollisionResponseToChannel` _staticmesh_2 "ECC_Visibility" "ECR_Block")
    (`PrimitiveComponent.SetCollisionResponseToChannel` _staticmesh_2 "ECC_GameTraceChannel1" "ECR_Block")
    (`PrimitiveComponent.SetSimulatePhysics` _staticmesh_2 true)))

(fn `OnRep_DefaultSkeletalMesh`
  (`SkeletalMeshComponent.SetSkeletalMeshAsset` (`self.SkeletalMesh`) (`self.DefaultSkeletalMesh`))
  (`SceneComponent.SetHiddenInGame` (`self.StaticMesh`) true false))

(fn `SaveObjectData_BPI`
  (params (SaveGame :type "/Game/SRPGE/Blueprints/Game/SaveLoad/BP_Game_Save Object Reference"))
  (returns (Success :type Boolean))
  (bind (_stackcount _ammocount _durability _decay) (break `/Game/SRPGE/Blueprints/Structures/Inventory/STR_ItemValues` (`.CurrentItemValues_68_EAF0DA8A4E892330842804B79249E216` (break `/Game/SRPGE/Blueprints/Structures/Inventory/STR_ItemData` (`self.Item`)))))
  ;[1 1 1] Sets save data
  (`KismetArrayLibrary.Array_Add` (`/Game/SRPGE/Blueprints/Game/SaveLoad/BP_Game_Save.ItemMasters` SaveGame) (make `/Game/SRPGE/Blueprints/Structures/SaveLoad/STR_SaveGame_ItemMaster` (`self.ItemGUID`) (`GameplayStatics.GetObjectClass` self) (`self.GetTransform`) (`self.Dropped`) (`self.ItemID`) _stackcount _ammocount _durability _decay))
  (return true))

(fn `SetRarity`
  (locals (LocalRarity :type Integer))
  (`|SwitchGameplayTag` (`.Rarity_40_4B3965C047BB0F1173541E9DE3438C00` (break `/Game/SRPGE/Blueprints/Structures/Inventory/STR_ItemData` (`self.Item`)))
    (:`Items.Rarity.Common`
      (set `self.RarityIndex` 2))
    (:`Items.Rarity.Uncommon`
      (set `self.RarityIndex` 3))
    (:`Items.Rarity.Rare`
      (set `self.RarityIndex` 4))
    (:`Items.Rarity.Epic`
      (set `self.RarityIndex` 5))
    (:`Items.Rarity.Legendary`
      (set `self.RarityIndex` 6)))
  (if (not (`self.AutoCollect`))
    (bind _returnvalue (`NiagaraFunctionLibrary.SpawnSystemAttached` "/Game/SRPGE/Demo/Assets/FXs/NS_ItemRarity.NS_ItemRarity" (`self.StaticMesh`) "None" (0.0 0.0 0.0) (struct) "KeepRelativeOffset"))
    (`/Engine/EditorBlueprintResources/StandardMacros.IsValid` _returnvalue
      (:`Is Valid`
        (`NiagaraComponent.SetVariableLinearColor` _returnvalue "Color" (select `int` (`self.RarityIndex`) :`0` (struct :`A` 1.0) :`1` (struct :`R` 1.0 :`G` 1.0 :`B` 1.0 :`A` 1.0) :`2` (struct :`R` 1.0 :`G` 1.0 :`B` 1.0 :`A` 1.0) :`3` (struct :`G` 1.0 :`B` 0.048172 :`A` 1.0) :`4` (struct :`G` 0.318547 :`B` 1.0 :`A` 1.0) :`5` (struct :`R` 0.672443 :`G` 0.14996 :`B` 1.0 :`A` 1.0) :`6` (struct :`R` 1.0 :`G` 0.291771 :`A` 1.0) :!type "LinearColor Structure"))))))

(fn `ShouldOutline_BPI`
  (returns (Outline :type Boolean) (CustomDepth :type Integer))
  (return true (`self.RarityIndex`)))

(fn `UserConstructionScript`
  ;[1 1 1] Sets default values for items placed in the world manually
  (set `self.ItemGUID` (`self.ActorGuid`))
  (if (not (`self.Dropped`))
    (`self.Set Item Data (Server)` (`self.ItemID`) (`self.StackCount`) (`self.AmmoCount`) (`self.Durability`) (`self.Decay`))))