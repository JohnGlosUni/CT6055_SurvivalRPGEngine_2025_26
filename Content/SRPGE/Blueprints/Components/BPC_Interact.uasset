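; Interaction component that lets players find and hold-to-use interactable objects, including a build refund mode.
; A looping timer on the local controller traces from camera or character to set the target, prompt widget and custom-depth outline.
; Hold time drives UI progress, while the server re-traces and triggers the interaction through interface messages.
; Targeted mesh instances listed in a data table get server-spawned harvestable actors, with their PCG points removed.
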(event Custom|InteractionTick
  ;[1 1 1] Sets the Interaction Tick using a timer.
  (if (Variables|Default|GetIsLocalController)
    (CallFunction|UpdateTarget)
    (CallFunction|CheckBuildRefund)
    (CallFunction|SetOutline)))

(event Custom|TryInteracting%20%28Client%29
  (params (InteractTime :type Float%20%28double-precision%29))
  (bind _target (Variables|Default|GetTarget))
  (bind _target_2 (Variables|Default|GetTarget))
  ;[1 1 1] Checks if the Target is an interactable object and passing the Trigger Interaction BPI after the trigger time defined for that interactable object.
  (if (and (Utilities|IsValid _target) (Utilities|DoesObjectImplementInterface _target "/Game/SRPGE/Blueprints/Interfaces/BPI_Interaction.BPI_Interaction_C"))
    (if (Variables|Default|GetFalseHold)
      (Variables|Default|SetInteractOffset InteractTime) ; Prevents the button from being pre-held before interacting with an object
      (Variables|Default|SetFalseHold false))
    (CallFunction|TryInteracting(Server) (- InteractTime (Variables|Default|GetInteractOffset)))
    (Utilities|IsValid _target_2
      (:Is%20Valid
        (bind (_caninteract _triggertime) (Class|BPIInteraction|CheckInteractableBPI(Message) _target_2))
        (if _caninteract
          (Class|BPIPlayerCharacter|UpdateInteractUIBPI(Message) (Components|GetOwner) (/ (- InteractTime (Variables|Default|GetInteractOffset)) _triggertime)))))
    (else
      (Variables|Default|SetFalseHold true))))

(event Custom|TryInteracting%20%28Server%29
  (params (InteractTime :type Float%20%28double-precision%29))
  ;[1 1 1] Checks if the Target is an interactable object and passing the Trigger Interaction BPI after the trigger time defined for that interactable object.
  (CallFunction|UpdateTarget)
  (if (not (Variables|Default|GetTriggered))
    (bind (_caninteract _triggertime) (Class|BPIInteraction|CheckInteractableBPI(Message) (Variables|Default|GetTarget)))
    (if (or (and (Variables|Default|GetBuildRefund) (>= InteractTime _triggertime)) (and _caninteract (>= InteractTime _triggertime)))
      (Variables|Default|SetTriggered true)
      (Class|BPIInteraction|TriggerInteractionBPI(Message) (Variables|Default|GetTarget) (Variables|Default|GetPlayer%20Controller) (Variables|Default|GetPlayer%20Character) (Variables|Default|GetBuildRefund))
      (Variables|Default|SetTarget 0))))

(event Custom|SpawnActor%20%28Server%29
  (params (HarvestableInfo :type STR%20Open%20World%20Interactables%20Structure%20%28by%20ref%29) (SpawnTransform :type Transform) (StaticMesh :type Static%20Mesh%20Object%20Reference) (PCGPoint :type PCG%20Point%20Structure))
  (bind (_harvestableclass _destroyclass _droptable) (Utilities|Struct|BreakSTR_OpenWorldInteractables HarvestableInfo))
  ;[1 1 1] Confirms hit actor on server and spawns it if valid. Passes PCG information for repsawning PCG points.
  (bind _hitresult (CallFunction|TickTrace))
  (if (.bBlockingHit (Collision|BreakHitResult _hitresult))
    (bind _player (Class|BPIPlayerCharacter|GetPlayerCharacterBPI(Message) (Components|GetOwner)))
    (bind _returnvalue (Game|SpawnActorfromClass _harvestableclass SpawnTransform "Undefined" "MultiplyWithRoot" 0 0))
    (Class|BPIInteraction|SetupHarvestableBPI(Message) _returnvalue -1.0 false _destroyclass 0.0 _droptable (Variables|/Script/Engine.Pawn|GetPlayerState _player) PCGPoint StaticMesh)
    (Class|BPIGameState|RemovePCGPointBPI(Message) (Game|GetGameState) PCGPoint)))

(event Custom|ResetInteraction%20%28Client%29
  ;[1 1 1] Checks if the Target is an interactable object and passing the Trigger Interaction BPI after the trigger time defined for that interactable object.
  (Class|BPIPlayerCharacter|UpdateInteractUIBPI(Message) (Components|GetOwner) 0.0)
  (Variables|Default|SetInteractOffset 0.0)
  (Variables|Default|SetFalseHold false))

(event Custom|ResetInteraction
  ;[1 1 1] Checks if the Target is an interactable object and passing the Trigger Interaction BPI after the trigger time defined for that interactable object.
  (Variables|Default|SetTriggered false))

(event Custom|SetBuildRefundMode%20%28Client%29
  (params (CanRefund :type Boolean))
  (bind _target (Variables|Default|GetTarget))
  ;[1 1 1] Sets Build Refund mode on Client and for the current target
  (Variables|Default|SetBuildRefund CanRefund)
  (Utilities|IsValid _target
    (:Is%20Valid
      (if (not (Variables|Default|GetBuildMove))
        (Class|BPIBuilding|SetBuildRefundBPI(Message) _target (Variables|Default|GetBuildRefund))))))

(event EventBeginPlay
  ;[1 1 1] Sets the Interaction Tick using a timer.
  (Utilities|Time|SetTimerbyEvent (delegate Custom|InteractionTick) 0.2 true))

(fn InitComponent
  (params (PlayerController :type Player%20Controller%20Object%20Reference) (PlayerCharacter :type BP%20Player%20Character%20Object%20Reference) (PlayerState :type BP%20Player%20State%20Object%20Reference))
  ;[1 1 1] Sets default values for interaction
  (Variables|Default|SetPlayer%20Character PlayerCharacter)
  (Utilities|IsValid PlayerController
    (:Is%20Valid
      (bind _output_get (Variables|Default|SetPlayer%20Controller PlayerController))
      (Variables|Default|SetIsLocalController (Utilities|IsValid (HUD|GetHUD _output_get)))
      (bind _asui_interaction (Utilities|Casting|CastToUI_Interaction (UserInterface|GetWidget (Variables|/Game/SRPGE/Blueprints/Player/BP_PlayerCharacter.BP_PlayerCharacter_C|GetInteractionWidget PlayerCharacter))))
      (Variables|Default|SetUI%20Interaction _asui_interaction)
      (EventDispatchers|BindEventtoOnBuildRefundMode PlayerState (EventDispatchers|CreateEvent :!event SetBuildRefundMode)))))

(fn UpdateTarget
  (bind _player_character (Variables|Default|GetPlayer%20Character))
  (bind _interactionwidget (Variables|/Game/SRPGE/Blueprints/Player/BP_PlayerCharacter.BP_PlayerCharacter_C|GetInteractionWidget _player_character))
  ;[1 1 1] Performs the Tick Trace and updates the Target if in range and hit.
  (Utilities|IsValid (Pawn|GetControlledPawn (Variables|Default|GetPlayer%20Controller))
    (:Is%20Valid
      (bind _hitresult (CallFunction|TickTrace))
      (if (.bBlockingHit (Collision|BreakHitResult _hitresult))
        (Variables|Default|SetImpact%20Normal (.ImpactNormal (Collision|BreakHitResult _hitresult)))
        (if (<= (Math|Vector|VectorLength (- (.Location (Collision|BreakHitResult _hitresult)) (Transformation|GetActorLocation (Pawn|GetControlledPawn (Variables|Default|GetPlayer%20Controller))))) (Variables|Default|GetHitDistance))
          (bind _caninteract (Class|BPIInteraction|CheckInteractableBPI(Message) (.HitActor (Collision|BreakHitResult _hitresult))))
          (Development|SetHiddeninGame _interactionwidget (not _caninteract) false)
          (bind (_text _hidebutton _offset) (Class|BPIInteraction|GetInteractionTextUIBPI(Message) (.HitActor (Collision|BreakHitResult _hitresult))))
          (Transformation|SetWorldLocation _interactionwidget (+ _offset (Transformation|GetActorLocation (.HitActor (Collision|BreakHitResult _hitresult)))) false false)
          (Default|UpdateName (Variables|Default|GetUI%20Interaction) _text _hidebutton)
          (CallFunction|SetTarget (.HitActor (Collision|BreakHitResult _hitresult)))
          (bind _asinstanced_static_mesh_component (Utilities|Casting|CastToInstancedStaticMeshComponent (.HitComponent (Collision|BreakHitResult _hitresult))))
          (bind _returnvalue (Utilities|GetDataTableRow "/Game/SRPGE/Blueprints/DataTables/DT_OpenWorldInteractables.DT_OpenWorldInteractables" (Utilities|String|StringToName (Utilities|GetObjectName (Variables|/Script/Engine.StaticMeshComponent|GetStaticMesh _asinstanced_static_mesh_component))))
            (:then
              (if (Utilities|Struct|BreakSTR_OpenWorldInteractables _returnvalue)
                (CallFunction|SpawnActor(Server) _returnvalue (.OutInstanceTransform (Components|InstancedStaticMesh|GetInstanceTransform _asinstanced_static_mesh_component (.HitItem (Collision|BreakHitResult _hitresult)) true)) (Variables|/Script/Engine.StaticMeshComponent|GetStaticMesh _asinstanced_static_mesh_component) (Utilities|Struct|MakePCGPoint (.OutInstanceTransform (Components|InstancedStaticMesh|GetInstanceTransform _asinstanced_static_mesh_component (.HitItem (Collision|BreakHitResult _hitresult)) true)))))))
          (else
            (CallFunction|SetTarget :!label _label)
            (Development|SetHiddeninGame (Variables|/Game/SRPGE/Blueprints/Player/BP_PlayerCharacter.BP_PlayerCharacter_C|GetInteractionWidget (Variables|Default|GetPlayer%20Character)) true false)))
        (else
          (goto _label))))))

(fn TickTrace
  (bind _player_controller (Variables|Default|GetPlayer%20Controller))
  (bind _player_character (Variables|Default|GetPlayer%20Character))
  (bind _playercameramanager (Variables|/Script/Engine.PlayerController|GetPlayerCameraManager _player_controller))
  (bind _mesh (Variables|/Script/Engine.Character|GetMesh _player_character))
  (bind _returnvalue (Camera|GetCameraLocation _playercameramanager))
  (bind _returnvalue_2 (Transformation|GetWorldLocation _mesh))
  (bind _returnvalue_3 (+ _returnvalue_2 "0.000000,0.000000,75.000000"))
  ;[1 1 1] Fires a trace from the camera that is looking for a new target.
  (LocalVariables|SetLocalDistance (Variables|Default|GetTraceDistance))
  (if (Variables|Default|GetTraceFromCamera)
    (bind _outhit (Collision|LineTraceByChannel _returnvalue (+ _returnvalue (* (Math|Vector|GetForwardVector (Camera|GetCameraRotation _playercameramanager)) (LocalVariables|GetLocalDistance))) "TraceTypeQuery1" false (Utilities|Array|MakeArray (Pawn|GetControlledPawn (Variables|Default|GetPlayer%20Controller))) "None")) ; Checks if anything is blocking (i.e. Wall) and updates Trace Distance accordingly
    (if (.bBlockingHit (Collision|BreakHitResult _outhit))
      (LocalVariables|SetLocalDistance (* (.Distance (Collision|BreakHitResult _outhit)) 1.2)))
    (bind _outhit_2 (Collision|SphereTraceByChannel _returnvalue (+ _returnvalue (* (Math|Vector|GetForwardVector (Camera|GetCameraRotation _playercameramanager)) (LocalVariables|GetLocalDistance))) 8.0 "TraceTypeQuery3" false (Utilities|Array|MakeArray (Pawn|GetControlledPawn (Variables|Default|GetPlayer%20Controller))) "None")) ; Larger Sphere Trace checks for interactables in an area
    (return _outhit_2)
    (else
      (bind _outhit_3 (Collision|SphereTraceByChannel _returnvalue_3 (+ _returnvalue_3 (* (Math|Vector|GetRightVector _mesh) (Variables|Default|GetPlayerTraceDistance))) 8e+01 "TraceTypeQuery3" false (Utilities|Array|MakeArray (Pawn|GetControlledPawn (Variables|Default|GetPlayer%20Controller)) (Variables|Default|GetPlayer%20Character)) "None"))
      (return _outhit_3))))

(fn SetTarget
  (params (NewTarget :type Actor%20Object%20Reference))
  ;[1 1 1] Sets the target and calls "On Target Changed"
  (if (!= NewTarget (Variables|Default|GetTarget))
    (Variables|Default|SetTarget NewTarget)))

(fn SetOutline
  (bind _target (Variables|Default|GetTarget))
  (bind _target_2 (Variables|Default|GetTarget))
  (bind _target_3 (Variables|Default|GetTarget))
  ;[1 1 1] Checks if the target should be outlined and outlines it if it should. If the target is no longer valid or the new target should not be outlined, removes the outline from the previous target.
  (Utilities|IsValid _target_3
    (:Is%20Valid
      (if (not (== _target_3 (Variables|Default|GetPreviousTarget)))
        (Utilities|IsValid (Variables|Default|GetPreviousTarget) :!label _label
          (:Is%20Valid
            (Class|BPIInteraction|LookingatBPI(Message) (Variables|Default|GetPreviousTarget) false (Variables|Default|GetPlayer%20Controller) (Variables|Default|GetPlayer%20Character))
            (bind _lookatserver (Class|BPIInteraction|GetLookatServerBPI(Message) (Variables|Default|GetPreviousTarget)))
            (if _lookatserver
              (bind _asbp_player_controller (Utilities|Casting|CastToBP_PlayerController (Variables|Default|GetPlayer%20Controller)))
              (Default|UpdateLookedat(Server) _asbp_player_controller (Variables|Default|GetPreviousTarget)))
            (for _array_element (Actor|GetComponentsByClass (Variables|Default|GetPreviousTarget) "/Script/Engine.PrimitiveComponent")
              (Rendering|SetRenderCustomDepth _array_element false)
              (Rendering|SetCustomDepthStencilValue _array_element 0)))
          (:Is%20Not%20Valid
            _))
        (Utilities|IsValid _target_2
          (:Is%20Valid
            (Class|BPIInteraction|LookingatBPI(Message) _target_2 true (Variables|Default|GetPlayer%20Controller) (Variables|Default|GetPlayer%20Character))
            (bind _lookatserver_2 (Class|BPIInteraction|GetLookatServerBPI(Message) (Variables|Default|GetTarget)))
            (if _lookatserver_2
              (bind _asbp_player_controller_2 (Utilities|Casting|CastToBP_PlayerController (Variables|Default|GetPlayer%20Controller)))
              (Default|UpdateLookedat(Server) _asbp_player_controller_2 (Variables|Default|GetPreviousTarget) (Variables|Default|GetTarget)))
            (Variables|Default|SetPreviousTarget _target)
            (bind (_outline _customdepth) (Class|BPIInteraction|ShouldOutlineBPI(Message) _target))
            (if _outline
              (for _array_element_2 (Actor|GetComponentsByClass _target "/Script/Engine.PrimitiveComponent")
                (Rendering|SetRenderCustomDepth _array_element_2 true)
                (Rendering|SetCustomDepthStencilValue _array_element_2 _customdepth))))
          (:Is%20Not%20Valid
            (Variables|Default|SetPreviousTarget 0)))))
    (:Is%20Not%20Valid
      (goto _label))))

(fn CheckBuildRefund
  (bind _target (Variables|Default|GetTarget))
  (if (not (Variables|Default|GetBuildMove))
    (if (Variables|Default|GetBuildRefund)
      (Utilities|IsValid _target
        (:Is%20Valid
          (if (not (== _target (Variables|Default|GetPreviousTarget)))
            (Class|BPIBuilding|SetBuildRefundBPI(Message) (Variables|Default|GetTarget) true)
            (Utilities|IsValid (Variables|Default|GetPreviousTarget) :!label _label
              (:Is%20Valid
                (Class|BPIBuilding|SetBuildRefundBPI(Message) (Variables|Default|GetPreviousTarget) false)))))
        (:Is%20Not%20Valid
          (goto _label))))))

(fn SetBuildRefundMode
  (params (CanDestroy :type Boolean))
  (Variables|Default|SetBuildRefund CanDestroy)
  (CallFunction|SetBuildRefundMode(Client) (Variables|Default|GetBuildRefund)))